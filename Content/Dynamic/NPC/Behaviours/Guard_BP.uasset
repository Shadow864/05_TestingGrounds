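; Guard_BP is an AI-controlled guard NPC that carries a gun and can take damage and die.
; Incoming damage reduces a clamped health value, and at zero the guard is flagged dead and detached from its controller.
; Each tick it sets an Aiming flag based on whether its AI controller has a valid focus actor.
; OnFire forwards the shot to the Gun_BP held in a child actor component.
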(event `self.ReceiveAnyDamage`
  (params (Damage :type "Float (single-precision)") (DamageType :type "DamageType Object Reference") (InstigatedBy :type "Controller Object Reference") (DamageCauser :type "Actor Object Reference"))
  (if (not (`self.IsDead`))
    (bind _output_get (set `self.Health` (`KismetMathLibrary.FClamp` (- (`self.Health`) Damage) 0.0 100.0)))
    (bind _output_get_2 (set `self.IsDead` (<= _output_get 0.0)))
    (if _output_get_2
      (`self.OnDie`))))

(event `self.ReceiveTick`
  (params (DeltaSeconds :type "Float (single-precision)"))
  (bind _asaicontroller (cast `AIController` (`self.GetController`)))
  (set `self.Aiming` (`KismetSystemLibrary.IsValid` (`AIController.GetFocusActor` _asaicontroller))))

(fn `OnDie`
  (`self.DetachFromControllerPendingDestroy`))

(fn `OnFire`
  (bind _asgun_bp (cast `/Game/Dynamic/Weapon/Behaviour/Gun_BP` (`ChildActorComponent.ChildActor` (`self.Gun`))))
  (`Gun.OnFire` _asgun_bp))

(fn `UserConstructionScript`)